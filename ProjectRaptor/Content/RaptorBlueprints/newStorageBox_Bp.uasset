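; Storage box actor that scores interactable items placed inside it and saves the total to a save slot.
; Box overlaps count any actor, highlight or unhighlight Interactable_Mesh_BP items, and add or subtract their item value.
; BeginPlay zeroes the saved score, and item overlaps write the running score to MySaveScore.
; A separate DoorStop trigger turns the point light green while a DoorHandle_BP overlaps it and red when it leaves.
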(event OnComponentBeginOverlap(Box)
  (params (OverlappedComponent :type Primitive%20Component%20Object%20Reference) (OtherActor :type Actor%20Object%20Reference) (OtherComp :type Primitive%20Component%20Object%20Reference) (OtherBodyIndex :type Integer) (bFromSweep :type Boolean) (SweepResult :type Hit%20Result%20Structure%20%28by%20ref%29))
  (bind _result (Math|Integer|IncrementInt (Variables|Default|GetItemCounter))
    (:%20%20
      (Variables|Default|SetItemCounter _result)
      (bind _asinteractable_mesh_bp (Utilities|Casting|CastToInteractable_Mesh_BP OtherActor))
      (Default|HighlightInteractable _asinteractable_mesh_bp)
      (CallFunction|AddtoScoreTally (.value (Variables|/Game/VirtualRealityBP/Blueprints/BP_PickupCube.BP_PickupCube_C|GetFItemInfo _asinteractable_mesh_bp)))
      (bind _returnvalue (SaveGame|LoadGamefromSlot "SlotName"))
      (bind _output_get (Variables|Default|SetSave _returnvalue))
      (bind _asmy_save_score (Utilities|Casting|CastToMySaveScore _output_get))
      (Variables|/Game/Spawn_BP/MySaveScore.MySaveScore_C|SetPointage _asmy_save_score (Variables|Default|GetCurrentScore))
      (SaveGame|SaveGametoSlot (Variables|Default|GetSave) "SlotName"))))

(event OnComponentEndOverlap(Box)
  (params (OverlappedComponent :type Primitive%20Component%20Object%20Reference) (OtherActor :type Actor%20Object%20Reference) (OtherComp :type Primitive%20Component%20Object%20Reference) (OtherBodyIndex :type Integer))
  (bind _result (Math|Integer|DecrementInt (Variables|Default|GetItemCounter))
    (:%20%20
      (Variables|Default|SetItemCounter _result)
      (bind _asinteractable_mesh_bp (Utilities|Casting|CastToInteractable_Mesh_BP OtherActor))
      (Default|Un-HighlightInteractable _asinteractable_mesh_bp)
      (CallFunction|RemovefromScoreTally (.value (Variables|/Game/Interactable_Mesh_BP.Interactable_Mesh_BP_C|GetFItemInfo _asinteractable_mesh_bp)))
      (bind _returnvalue (SaveGame|LoadGamefromSlot "SlotName"))
      (bind _output_get (Variables|Default|SetSave _returnvalue))
      (bind _asmy_save_score (Utilities|Casting|CastToMySaveScore _output_get))
      (Variables|/Game/Spawn_BP/MySaveScore.MySaveScore_C|SetPointage _asmy_save_score (Variables|Default|GetCurrentScore))
      (SaveGame|SaveGametoSlot (Variables|Default|GetSave) "SlotName"))))

(event OnComponentBeginOverlap(DoorStop)
  (params (OverlappedComponent :type Primitive%20Component%20Object%20Reference) (OtherActor :type Actor%20Object%20Reference) (OtherComp :type Primitive%20Component%20Object%20Reference) (OtherBodyIndex :type Integer) (bFromSweep :type Boolean) (SweepResult :type Hit%20Result%20Structure%20%28by%20ref%29))
  (if (== (Utilities|GetClass OtherActor) "/Game/DoorHandle_BP.DoorHandle_BP_C")
    (Development|PrintString "DoorEngaged")
    (Rendering|Components|Light|SetLightColor (Variables|Default|GetPointLight) "(R=0.064762,G=0.887923,B=0.031535,A=1.000000)" true)))

(event OnComponentEndOverlap(DoorStop)
  (params (OverlappedComponent :type Primitive%20Component%20Object%20Reference) (OtherActor :type Actor%20Object%20Reference) (OtherComp :type Primitive%20Component%20Object%20Reference) (OtherBodyIndex :type Integer))
  (if (== (Utilities|GetClass OtherActor) "/Game/DoorHandle_BP.DoorHandle_BP_C")
    (Development|PrintString "DoorEngaged")
    (Rendering|Components|Light|SetLightColor (Variables|Default|GetPointLight) "(R=0.863157,G=0.038204,B=0.051269,A=1.000000)" true)))

(event EventBeginPlay
  (Variables|Default|SetItemCounter 0)
  (Variables|Default|SetCurrentScore 0.0)
  (bind _returnvalue (SaveGame|LoadGamefromSlot "SlotName"))
  (bind _output_get (Variables|Default|SetSave _returnvalue))
  (bind _asmy_save_score (Utilities|Casting|CastToMySaveScore _output_get))
  (Variables|/Game/Spawn_BP/MySaveScore.MySaveScore_C|SetPointage _asmy_save_score (Variables|Default|GetCurrentScore))
  (SaveGame|SaveGametoSlot (Variables|Default|GetSave) "SlotName"))

(event EventTick
  (params (DeltaSeconds :type Float%20%28single-precision%29))
  (Variables|Default|SetElapsedTime (+ DeltaSeconds (Variables|Default|GetElapsedTime))))

(fn ConstructionScript)

(fn AddtoScoreTally
  (params (valueewParam :type Float%20%28single-precision%29))
  (Variables|Default|SetCurrentScore (+ valueewParam (Variables|Default|GetCurrentScore))))

(fn RemovefromScoreTally
  (params (value :type Float%20%28single-precision%29))
  (Variables|Default|SetCurrentScore (- (Variables|Default|GetCurrentScore) value)))