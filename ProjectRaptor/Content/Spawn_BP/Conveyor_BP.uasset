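; Conveyor belt actor that carries interactable meshes along its forward direction, pausing for any the player is holding.
; Each tick it casts the actors overlapping its Box to Interactable_Mesh_BP and skips motion controllers and grabbed meshes.
; The rest get an unswept world offset scaled by delta time and a speed set on BeginPlay.
; The offset targets both the array element and its cast reference, the same actor.
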(event EventTick
  (params (DeltaSeconds :type Float%20%28single-precision%29))
  (for _array_element (Collision|GetOverlappingActors (Variables|Default|GetBox) 0 :!class /Script/Engine.PrimitiveComponent)
    (bind _asinteractable_mesh_bp (Utilities|Casting|CastToInteractable_Mesh_BP _array_element))
    (if (not (== (Utilities|GetClass _array_element) "/Game/VirtualRealityBP/Blueprints/BP_MotionController.BP_MotionController_C"))
      (if (not (Variables|/Game/Interactable_Mesh_BP.Interactable_Mesh_BP_C|GetisGrabbed _asinteractable_mesh_bp))
        (Transformation|AddActorWorldOffset _array_element (* (Math|Vector|GetForwardVector (Transformation|GetActorRotation)) (* DeltaSeconds (Variables|Default|GetSpeed))))))))

(event EventBeginPlay
  (Variables|Default|SetSpeed 2e+02))

(fn ConstructionScript)