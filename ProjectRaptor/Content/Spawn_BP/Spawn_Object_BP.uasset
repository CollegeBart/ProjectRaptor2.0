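; Timed spawner Blueprint that repeatedly spawns a random actor class from the ToSpawn array at the location of a referenced SpawnPoint actor.
; Tick accumulates delta time in TimePassed and, once it exceeds Delay, resets it and spawns one actor.
; Spawns use only the point's location, with zero rotation and unit scale, and ignore collisions.
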(event EventTick
  (params (DeltaSeconds :type Float%20%28single-precision%29))
  (bind _to_spawn (Variables|Default|GetTo_Spawn))
  (bind _output_get (Variables|Default|SetTime_passed (+ DeltaSeconds (Variables|Default|GetTime_passed))))
  (Math|Float|CompareFloat _output_get (Variables|Default|GetDelay)
    (:>
      (Utilities|FlowControl|Sequence
        (:then_0
          (Variables|Default|SetTime_passed 0.0))
        (:then_1
          (Game|SpawnActorfromClass (Utilities|Array|Get(acopy) _to_spawn (Math|Random|RandomInteger (Utilities|Array|Length _to_spawn))) (Math|Transform|MakeTransform (Transformation|GetActorLocation (Variables|Default|GetSpawn_Point))) "AlwaysSpawn" 0 0))))))

(fn ConstructionScript)